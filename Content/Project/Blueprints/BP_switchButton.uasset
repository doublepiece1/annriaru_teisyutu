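; Floor or wall switch button that, when BP_Player overlaps its trigger box, opens a linked door and/or starts a linked moving box.
; The SwitchOn timeline animates the button mesh's Z, then calls OpenDoor on TargetDoor and activates TargetBox's InterpToMovement, each if valid.
; Only the door path calls the SetEventFinished override, which runs the parent logic, zeroes the button's relative location and disables trigger collision.
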(event `self.Box.OnComponentBeginOverlap`
  (params (OverlappedComponent :type "PrimitiveComponent Object Reference") (OtherActor :type "Actor Object Reference") (OtherComp :type "PrimitiveComponent Object Reference") (OtherBodyIndex :type Integer) (bFromSweep :type Boolean) (SweepResult :type "HitResult Structure (by ref)"))
  (cast `/Game/Project/Blueprints/BP_Player` OtherActor)
  (bind (_direction _buttonz) (`Timeline|SwitchOn`)
    (:`Update`
      (`SceneComponent.K2_SetRelativeLocation` (`self.STM_Button`) (`KismetMathLibrary.MakeVector` 0.0 0.0 _buttonz) false false))
    (:`Finished`
      (`|ExecutionSequence`
        (:`then_0`
          (bind _target_door (`self.Target Door`)
            (:`then`
              (`/Game/Project/Blueprints/BP_Door.OpenDoor` _target_door)
              (`self.SetEventFinished`))
            (:`else`)))
        (:`then_1`
          (bind _target_box (`self.Target Box`)
            (:`then`
              (`ActorComponent.SetActive` (`/Game/Project/Blueprints/BP_MovingBox.InterpToMovement` _target_box) true false))
            (:`else`)))))))

(event `self.ReceiveBeginPlay`
  (`parent.ReceiveBeginPlay`))

(fn `NewFunction`
  (set `self.Target Box` null))

(fn `SetEventFinished`
  (`parent.SetEventFinished`)
  (`SceneComponent.K2_SetRelativeLocation` (`self.STM_Button`) (0.0 0.0 0.0) false false)
  (`PrimitiveComponent.SetCollisionEnabled` (`self.Box`) "NoCollision"))

(fn `UserConstructionScript`)