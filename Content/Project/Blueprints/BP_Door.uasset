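; Door actor that swings open when the player overlaps its Box, optionally requiring a key.
; Keyless doors open unless flagged SwitchDoor; otherwise the GameInstance key status must be Got, and is saved as Used on opening.
; OpenDoor clears SwitchDoor and drives the mesh yaw through a Timeline.
; SetEventFinished, extending the parent's version, snaps the door open and disables Box collision.
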(event `self.ReceiveBeginPlay`
  (`parent.ReceiveBeginPlay`))

(event `OpenDoor`
  (set `self.SwitchDoor` false)
  (bind (_direction _openz) (`Timeline|タイムライン`)
    (:`Update`
      (`SceneComponent.K2_SetRelativeRotation` (`self.STM_Door`) (`KismetMathLibrary.MakeRotator` 0.0 0.0 _openz) false false))
    (:`Finished`
      (`self.SetEventFinished`))))

(event `self.Box.OnComponentBeginOverlap`
  (params (OverlappedComponent :type "PrimitiveComponent Object Reference") (OtherActor :type "Actor Object Reference") (OtherComp :type "PrimitiveComponent Object Reference") (OtherBodyIndex :type Integer) (bFromSweep :type Boolean) (SweepResult :type "HitResult Structure (by ref)"))
  (if (`ActorComponent.ComponentHasTag` OtherComp "Player")
    (if (and (== (`self.KeyName`) "None") (not (`self.SwitchDoor`)))
      (`self.OpenDoor`)
      (else
        (switch `/Game/Project/Blueprints/EN_KeyStatus` (`/Game/Project/Blueprints/BP_MyGameinstance.GetKeyStatus` (`self.My Game Instance`) (`self.KeyName`))
          (:`NewEnumerator1`
            (`/Game/Project/Blueprints/BP_MyGameinstance.SaveKeyStatus` (`self.My Game Instance`) (`self.KeyName`) "NewEnumerator2")
            (`self.OpenDoor`)))))))

(fn `SetEventFinished`
  (`parent.SetEventFinished`)
  (set `self.SwitchDoor` false)
  (`SceneComponent.K2_SetRelativeRotation` (`self.STM_Door`) (struct :`Yaw` 90.0) false false)
  (`PrimitiveComponent.SetCollisionEnabled` (`self.Box`) "NoCollision"))

(fn `UserConstructionScript`)