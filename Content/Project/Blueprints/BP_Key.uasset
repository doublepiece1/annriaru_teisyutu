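; BP_Key is a key pickup actor, derived from a parent that provides a SetEventFinished hook.
; When a component tagged Player overlaps its Sphere, it notifies the player through ACOverlapPlayer with the key name and saves that key's status in the game instance.
; It then calls SetEventFinished, which runs the parent logic and destroys the actor.
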(event `self.Sphere.OnComponentBeginOverlap`
  (params (OverlappedComponent :type "PrimitiveComponent Object Reference") (OtherActor :type "Actor Object Reference") (OtherComp :type "PrimitiveComponent Object Reference") (OtherBodyIndex :type Integer) (bFromSweep :type Boolean) (SweepResult :type "HitResult Structure (by ref)"))
  (if (`ActorComponent.ComponentHasTag` OtherComp "Player")
    (`/Game/Project/Blueprints/AC_OverlapPlayer.NotifyToPlayer` (`self.AC_OverlapPlayer`) OtherActor (`self.KeyName`))
    (`/Game/Project/Blueprints/BP_MyGameinstance.SaveKeyStatus` (`self.My Game Instance`) (`self.KeyName`) "NewEnumerator1")
    (`self.SetEventFinished`)))

(event `self.ReceiveBeginPlay`
  (`parent.ReceiveBeginPlay`))

(fn `SetEventFinished`
  (`parent.SetEventFinished`)
  (`self.K2_DestroyActor`))

(fn `UserConstructionScript`)