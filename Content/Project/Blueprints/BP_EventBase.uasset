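; BP_EventBase is a base Blueprint for game events whose completion status persists through BP_MyGameinstance.
; The construction script derives each event's name from its display name, which serves as the save key.
; On BeginPlay it reads the saved status, calling SetEventFinished for finished events and resetting any other to Default.
; SetEventFinished marks the event Finished and writes that status back to the game instance.
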(event `self.ReceiveBeginPlay`
  (bind _asbp_my_gameinstance (cast `/Game/Project/Blueprints/BP_MyGameinstance` (`GameplayStatics.GetGameInstance`)))
  (bind _output_get (set `self.My Game Instance` _asbp_my_gameinstance))
  (bind _output_get_2 (set `self.EventStatus` (`/Game/Project/Blueprints/BP_MyGameinstance.GetEventStatus` _output_get (`self.Event Name`))))
  (switch `/Game/Project/Blueprints/EN_EventStatus` _output_get_2
    (:`NewEnumerator0`
      (bind _output_get_3 (set `self.EventStatus` "NewEnumerator0"))
      (`/Game/Project/Blueprints/BP_MyGameinstance.SaveEventStatus` (`self.My Game Instance`) (`self.Event Name`) _output_get_3))
    (:`NewEnumerator2`
      (`self.SetEventFinished`))))

(fn `SetEventFinished`
  (bind _output_get (set `self.EventStatus` "NewEnumerator2"))
  (`/Game/Project/Blueprints/BP_MyGameinstance.SaveEventStatus` (`self.My Game Instance`) (`self.Event Name`) _output_get))

(fn `UserConstructionScript`
  (set `self.Event Name` (`KismetStringLibrary.Conv_StringToName` (`KismetSystemLibrary.GetDisplayName` self))))